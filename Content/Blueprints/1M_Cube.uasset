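; Collectible cube actor that acts as a key pickup, with a point light as highlight.
; Tick zeroes the light every frame and voirblock raises it, so the glow lasts only while that event keeps being called.
; The rammaser_object event increments NbClefs (key count) on the player's ThirdPersonCharacter, then destroys the cube.
; Neither custom event is triggered within this Blueprint.
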(event Custom|voir%20block
  (Rendering|Components|Light|SetIntensity (Variables|Default|GetPointLight) 1e+02))

(event Custom|rammaser_object
  (bind _asthird_person_character (Utilities|Casting|CastToThirdPersonCharacter (Game|GetPlayerCharacter 0)))
  (bind _result (Math|Integer|IncrementInt (Variables|/Game/ThirdPersonBP/Blueprints/ThirdPersonCharacter.ThirdPersonCharacter_C|Getnb_clefs _asthird_person_character))
    (:%20%20
      (Variables|/Game/ThirdPersonBP/Blueprints/ThirdPersonCharacter.ThirdPersonCharacter_C|Setnb_clefs _asthird_person_character _result)
      (Actor|DestroyActor))))

(event EventBeginPlay)

(event Collision|EventActorBeginOverlap
  (params (OtherActor :type Actor%20Object%20Reference)))

(event EventTick
  (params (DeltaSeconds :type Float%20%28single-precision%29))
  (Rendering|Components|Light|SetIntensity (Variables|Default|GetPointLight) 0.0))

(fn ConstructionScript)